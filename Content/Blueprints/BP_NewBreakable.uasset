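; Breakable walkable floor tile for click-to-move pathing that cracks and shakes when stepped on, then drops away when stepped off.
; Hover and Interact drive character pathing, while breaking blocks the Walkable and disables the trigger box.
; A day/night switch on a cracked tile drops the player with it and restarts the stage.
; Broken tiles count switches, then rebuild by reversing the fall timeline, also triggered by ResetFloor.
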(event `/Game/Prototyping/Interact/InteractInterface.Interact`
  ;[0 0 0] Run on mouseover and click
  (`/Game/Blueprints/Characters/GP2_PlayerCharacter.MoveAlongPath` (`/Game/Core/BFL_Core.GetCharacter`)))

(event `/Game/Prototyping/Interact/InteractInterface.Hover`
  ;[0 0 0] Run on mouseover and click
  (`PlayerCharacter.GeneratePathToWalkable` (`/Game/Core/BFL_Core.GetCharacter`) self))

(event `self.ReceiveBeginPlay`
  ;[0 0 0] Begin Play
  ;[0 0 0] Set startLocation for timeline lerp
  (set `self.StartingLocation` (`SceneComponent.K2_GetComponentLocation` (`self.Cube`))))

(event `/Game/Movement/PathInterface.UpdatePathData`
  ;[0 0 0 1 24] Update Path
  (set `/Game/Movement/PathComponent.PathType` (select `bool` (`WalkableComponent.blocked` (`self.Walkable`)) :`false` "NewEnumerator0" :`true` "NewEnumerator1" :!type "/Game/Movement/E_PathPointTypes Enum") (`self.PathComponent`)))

(event `/Game/Core/BPI_LevelReset.ResetFloor`
  (bind _startinglocation (`self.StartingLocation`))
  (bind _startinglocation_2 (`self.StartingLocation`))
  (if (`self.Broken`)
    ;[0 0 0] Rebuild after x turns
    (`self.Stop Shaky` :!label _label)
    (set `self.RebuildingTurns` 0)
    (set `self.Broken` false)
    (set `self.Cracked` false)
    (set `WalkableComponent.blocked` false (`self.Walkable`))
    (set `self.PlayerFall` false)
    (`PrimitiveComponent.SetCollisionEnabled` (`self.Box`) "QueryOnly")
    (`SceneComponent.SetVisibility` (`self.Cube`) true false)
    ;[0 0 0] Break when stepped of
    (bind (_direction _alpha) (`Timeline|Timeline_0` :!via `ReverseFromEnd` :!label _label_2)
      (:`Update`
        (`SceneComponent.K2_SetWorldLocation` (`self.Cube`) (`KismetMathLibrary.VLerp` _startinglocation (`KismetMathLibrary.MakeVector` (.x _startinglocation) (.y _startinglocation) (- (.z _startinglocation) 5000.0)) _alpha) false false)
        (if (`self.PlayerFall`)
          (`SceneComponent.K2_SetWorldLocation` (`Actor.RootComponent` (`/Game/Core/BFL_Core.GetCharacter`)) (`KismetMathLibrary.VLerp` _startinglocation_2 (`KismetMathLibrary.MakeVector` (.x _startinglocation_2) (.y _startinglocation_2) (- (.z _startinglocation_2) 2000.0)) _alpha) false false)))
      (:`Finished`
        (if (`self.Broken`)
          (`SceneComponent.SetVisibility` (`self.Cube`) false false))
        (if (`self.PlayerFall`)
          (`/Game/Blueprints/Characters/GP2_PlayerCharacter.Restart Stage` (`/Game/Core/BFL_Core.GetCharacter`))
          (set `self.PlayerFall` false))))))

(event `self.DayNightTrigger.onDay`
  (params (time :type Integer))
  ;[0 0 0] Rebuild after x turns
  (if (`self.Broken`) :!label _label_3
    (bind _result (`/Engine/EditorBlueprintResources/StandardMacros.IncrementInt` (`self.RebuildingTurns`))
      (:`  `
        (if (>= _result (`self.RebuildTurnDelay`))
          (goto _label))))
    (else
      ;[0 0 0] Fall if changing day/night and is cracked
      (if (`self.Cracked`)
        (set `self.PlayerFall` true)
        ;[0 0 0] Break when stepped of
        (`PrimitiveComponent.SetCollisionEnabled` (`self.Box`) "NoCollision" :!label _label_4)
        (`|ExecutionSequence`
          (:`then_0`
            (set `WalkableComponent.blocked` true (`self.Walkable`))
            (set `self.Broken` true)
            (goto _label_2 :!via `PlayFromStart`))
          (:`then_1`
            (`self.Stop Shaky`)))))))

(event `self.DayNightTrigger.onNight`
  (params (time :type Integer))
  ;[0 0 0] Rebuild after x turns
  (goto _label_3))

(event `self.Box.OnComponentEndOverlap`
  (params (OverlappedComponent :type "PrimitiveComponent Object Reference") (OtherActor :type "Actor Object Reference") (OtherComp :type "PrimitiveComponent Object Reference") (OtherBodyIndex :type Integer))
  ;[0 0 0] Break when stepped of
  (goto _label_4))

(event `self.Box.OnComponentBeginOverlap`
  (params (OverlappedComponent :type "PrimitiveComponent Object Reference") (OtherActor :type "Actor Object Reference") (OtherComp :type "PrimitiveComponent Object Reference") (OtherBodyIndex :type Integer) (bFromSweep :type Boolean) (SweepResult :type "HitResult Structure (by ref)"))
  (bind (_relativelocation_x _relativelocation_y _relativelocation_z) (`KismetMathLibrary.BreakVector` (`SceneComponent.RelativeLocation` (`self.Cube`))))
  ;[0 0 0] Change material and crack when stepped on
  (set `self.Cracked` true)
  (`|ExecutionSequence`
    (:`then_0`
      (bind (_direction _alpha) (`Timeline|TL_Shaky` :!via `PlayFromStart` :!label _label_5)
        (:`Update`
          (`SceneComponent.K2_SetRelativeLocation` (`self.Cube`) (`KismetMathLibrary.MakeVector` _relativelocation_x (`KismetMathLibrary.Lerp` -20.0 20.0 _alpha) _relativelocation_z) false false))
        (:`Finished`
          (`KismetSystemLibrary.Delay` 0.1)
          (`/Engine/EditorBlueprintResources/StandardMacros.Gate` false :!label _label_6
            (:`Exit`
              (goto _label_5 :!via `PlayFromStart`))))))
    (:`then_1`
      (goto _label_6 :!via `Open`))))

(event `Stop Shaky`
  (`|ExecutionSequence`
    (:`then_0`
      (goto _label_5 :!via `Stop`))
    (:`then_1`
      (goto _label_6 :!via `Close`))))

(fn `GetInteractTransform`
  (returns (Transform :type "Transform Structure"))
  (return (`SceneComponent.K2_GetComponentToWorld` (`self.WalkToPosition`))))

(fn `GetPathPoint`
  (returns (PathPoint :type "Vector Structure"))
  (return (`SceneComponent.K2_GetComponentLocation` (`self.WalkToPosition`))))

(fn `UserConstructionScript`)