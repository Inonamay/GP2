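; Player character Blueprint for tile-based movement paid for with action points, which replenish at day and night.
; Gated events store the found path, then walk it tile by tile until it ends, is interrupted or points run out.
; Movement start, step and end are broadcast to actors and widgets through MovementInterface.
; RestartStage handles death, clearing key items, floating the player to the starting tile by timeline and restoring key item pickups.
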(event `Restart Stage`
  (bind _startingtile (`self.startingTile`))
  (bind _startingtile_2 (`self.startingTile`))
  ;[0 0 0 1 42] Move Player back to stage starting tile on death
  (`/Game/Movement/BFL_Movement.BlockOpenMovement` "NewEnumerator1")
  (`KismetArrayLibrary.Array_Clear` (`self.Path`))
  (`self.SetCurrentTile` _startingtile)
  (set `self.DeathLocaiton` (`self.K2_GetActorLocation`))
  (bind _transform (message `/Game/Prototyping/Interact/InteractInterface.GetInteractTransform` _startingtile))
  (bind _returnvalue (`GameplayStatics.SpawnEmitterAttached` "/Game/Particles/P_Bubbles.P_Bubbles" (`self.Mesh`) "None" (0.0 0.0 200.0) (struct) (1.5 1.5 1.5)))
  (`self.SetActorEnableCollision` false)
  (set `self.KeyItems` 0)
  ;;[0.276 0.276 0.276] Update HUD
  (bind _asgp2player_controller (cast `/Game/Core/GP2PlayerController` (`GameplayStatics.GetPlayerController` 0)))
  (`/Game/HUD/UI_KeyItemCount.Update Item` (`/Game/HUD/MainHUD.UI_KeyItemCount` (`/Game/Core/GP2PlayerController.Main HUD` _asgp2player_controller)))
  (bind (_direction _alpha _height) (`Timeline|TL_ResetPlayer` :!via `PlayFromStart`)
    (:`Update`
      (`self.K2_SetActorLocation` (`KismetMathLibrary.VLerp` (`KismetMathLibrary.MakeVector` (.x (`self.DeathLocaiton`)) (.y (`self.DeathLocaiton`)) (+ (.z (`self.DeathLocaiton`)) 100.0)) (+ (.location _transform) _height) _alpha)))
    (:`Finished`
      (`self.SetActorEnableCollision` true)
      (`ActorComponent.K2_DestroyComponent` _returnvalue)
      (bind _outactors (`GameplayStatics.GetAllActorsOfClass` "/Game/Prototyping/TowerIsland/BP_Keyitem.BP_Keyitem_C"))
      (for _array_element _outactors
        (bind _staticmesh (`/Game/Prototyping/TowerIsland/BP_Keyitem.StaticMesh` _array_element))
        (`PrimitiveComponent.SetCollisionEnabled` _staticmesh "QueryOnly")
        (`SceneComponent.SetVisibility` _staticmesh true false)
        (`self.SetCurrentTile` _startingtile_2)
        (set `self.TargetTile` _startingtile_2)
        (`/Game/Movement/BFL_Movement.BlockOpenMovement` "NewEnumerator0")))))

(event `Action Failed` :!signature `self.actionFailed`
  (params (errorType :type "ActionError Enum" :default "NoPath"))
  (`KismetSystemLibrary.PrintString` (`|GetEnumeratorNameAsString` errorType)))

(event `self.DayNightTrigger.onDay`
  (params (time :type Integer))
  ;[0 0 0] Day/night
  (`self.ReplenishActionPoints` 4))

(event `self.ReceiveTick`
  (params (DeltaSeconds :type "Float (single-precision)"))
  ;[1 0 0] DEBUG!!
)

(event `self.ReceiveBeginPlay`
  ;[0 0 0 1 32] Begin Play
  (set `self.startingTile` (`self.Tile`))
  (add `self.onFoundPath` (delegate `OnPathFound`))
  (add `self.actionFailed` (delegate `Action Failed`)))

(event `self.DayNightTrigger.onNight`
  (params (time :type Integer))
  ;[0 0 0] Day/night
  (`self.ReplenishActionPoints` 4))

(event `OnPathFound` :!signature `self.onFoundPath`
  (params (path :type "Array of Actor Object Reference (by ref)") (actionPointCost :type Integer))
  ;[0 0 0 1 24] Set new Path from OnPathFound script
  (`/Engine/EditorBlueprintResources/StandardMacros.Gate` false :!label _label
    (:`Exit`
      (bind _output_get (set `self.Path` path))
      (set `self.TargetTile` (`|GetArrayItem` _output_get (`KismetArrayLibrary.Array_LastIndex` _output_get))) ; Save the last tile in path
      (`KismetArrayLibrary.Array_Remove` _output_get) ; Remove the tile we are already standing on
    )))

(event `OpenPathFoundGate`
  ;[0 0 0 1 24] Set new Path from OnPathFound script
  (goto _label :!via `Open`))

(event `ClosePathFoundGate`
  ;[0 0 0 1 24] Set new Path from OnPathFound script
  (goto _label :!via `Close`))

(event `MoveAlongPath`
  (bind _returnvalue (`self.GetActionPoints`))
  (bind _path (`self.Path`))
  (bind _output (`|GetArrayItem` _path))
  ;[0 0 0] Check if player can move
  (`/Engine/EditorBlueprintResources/StandardMacros.Gate` false :!label _label_2
    (:`Exit`
      (if (== (`self.GetActionPoints`) 0)
        _
        (elif (not (`self.Moving`))
          ;;[0 0 0] Close pathfinding and movement when moving
          (`self.ClosePathFoundGate`)
          (`self.CloseMoveGate`)
          ;[0 0 0 1 32] Run Player movement
          (`|ExecutionSequence`
            (:`then_0`
              ;;[0 0 0] Broadcast MovementStarted to Widgets and Actors with Interface
              (set `self.Moving` true)
              (bind _outactors (`GameplayStatics.GetAllActorsWithInterface` "/Game/Movement/MovementInterface.MovementInterface_C"))
              (for _array_element _outactors
                (message `/Game/Movement/MovementInterface.MovingStarted` _array_element))
              (bind _foundwidgets (`WidgetBlueprintLibrary.GetAllWidgetsWithInterface` "/Game/Movement/MovementInterface.MovementInterface_C"))
              (for _array_element_2 _foundwidgets
                (message `/Game/Movement/MovementInterface.MovingStarted` _array_element_2)))
            (:`then_1`
              ;;[0 0 0] Check if there is a step left to take
              (if (and (`KismetArrayLibrary.Array_IsValidIndex` _path) (not (`self.InterrupMovement`))) :!label _label_3
                ;;[0 0 0] Check if player has enough action points
                (bind _returnvalue_2 (`self.DoAction` (`WalkableComponent.pointsCost` (`/Game/Core/BFL_Core.GetWalkable` _output))))
                (if _returnvalue_2
                  ;[1 0 0] Temp Fix!
                  (if (and (> (`KismetArrayLibrary.Array_Length` _path) _returnvalue) (<= _returnvalue 2))
                    (`self.SetCurrentTile` _output))
                  (`SkeletalMeshComponent.PlayAnimation` (`self.Mesh`) "/Game/Blueprints/Characters/Lucy/Animations/AM_Lucy_Transition_01.AM_Lucy_Transition_01" false)
                  (`KismetSystemLibrary.Delay` 0.2)
                  ;;[0 0 0] Move Player to next Tile
                  (bind _transform (message `/Game/Prototyping/Interact/InteractInterface.GetInteractTransform` _output))
                  (`KismetSystemLibrary.MoveComponentTo` (`self.CapsuleComponent`) (.location _transform) (`self.K2_GetActorRotation`) true true)
                  ;;[0 0 0] remove step taken from path
                  (`KismetArrayLibrary.Array_Remove` _path)
                  ;;[0 0 0] Broadcast Player Moved one step to Widgets and Actors with Interface
                  (bind _outactors_2 (`GameplayStatics.GetAllActorsWithInterface` "/Game/Movement/MovementInterface.MovementInterface_C"))
                  (for _array_element_3 _outactors_2
                    (message `/Game/Movement/MovementInterface.MovedOneStep` _array_element_3))
                  (bind _foundwidgets_2 (`WidgetBlueprintLibrary.GetAllWidgetsWithInterface` "/Game/Movement/MovementInterface.MovementInterface_C"))
                  (for _array_element_4 _foundwidgets_2
                    (message `/Game/Movement/MovementInterface.MovedOneStep` _array_element_4))
                  ;;[0 0 0] Stay at tile before checking if player can move another
                  (`KismetSystemLibrary.Delay` 0.2)
                  (goto _label_3)
                  (else
                    (`self.End Movement` true)))
                (else
                  (`self.End Movement` false))))))))))

(event `OpenMoveGate`
  ;[0 0 0] Check if player can move
  (goto _label_2 :!via `Open`))

(event `CloseMoveGate`
  ;[0 0 0] Check if player can move
  (goto _label_2 :!via `Close`))

(event `End Movement`
  (params (EndEarly :type Boolean))
  ;[0 0 0 1 32] End Movement
  (if (not EndEarly)
    (`self.SetCurrentTile` (`self.TargetTile`)))
  (`SkeletalMeshComponent.SetAnimationMode` (`self.Mesh`) "AnimationBlueprint")
  ;;[0 0 0] Broadcast MovementEnded
  (bind _outactors (`GameplayStatics.GetAllActorsWithInterface` "/Game/Movement/MovementInterface.MovementInterface_C"))
  (for _array_element _outactors
    (message `/Game/Movement/MovementInterface.MovingEnded` _array_element))
  (bind _foundwidgets (`WidgetBlueprintLibrary.GetAllWidgetsWithInterface` "/Game/Movement/MovementInterface.MovementInterface_C"))
  (for _array_element_2 _foundwidgets
    (message `/Game/Movement/MovementInterface.MovingEnded` _array_element_2)
    (set `self.Moving` false)
    (if (`self.InterrupMovement`)
      (set `self.InterrupMovement` false)
      (else
        (`self.OpenPathFoundGate`)
        (`self.OpenMoveGate`)))))

(fn `UserConstructionScript`)