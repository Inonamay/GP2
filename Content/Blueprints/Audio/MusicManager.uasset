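; MusicManager is an audio Blueprint that starts the music on BeginPlay and changes it according to location and time of day.
; Six overlap components, Track01 to Track06, each call SwitchTrack with their number and print a debug label, without filtering the overlapping actor.
; DayNightTrigger events call AddLayer at night and RemoveLayer by day.
; The bodies of these music functions are not in this file.
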(event `self.DayNightTrigger.onDay`
  (params (time :type Integer))
  (`self.RemoveLayer`))

(event `self.DayNightTrigger.onNight`
  (params (time :type Integer))
  (`self.AddLayer`))

(event `self.ReceiveBeginPlay`
  (`self.StartMusic`))

(event `self.Track01.OnComponentBeginOverlap`
  (params (OverlappedComponent :type "PrimitiveComponent Object Reference") (OtherActor :type "Actor Object Reference") (OtherComp :type "PrimitiveComponent Object Reference") (OtherBodyIndex :type Integer) (bFromSweep :type Boolean) (SweepResult :type "HitResult Structure (by ref)"))
  (`self.SwitchTrack` 1)
  (`KismetSystemLibrary.PrintString` "Track01"))

(event `self.Track02.OnComponentBeginOverlap`
  (params (OverlappedComponent :type "PrimitiveComponent Object Reference") (OtherActor :type "Actor Object Reference") (OtherComp :type "PrimitiveComponent Object Reference") (OtherBodyIndex :type Integer) (bFromSweep :type Boolean) (SweepResult :type "HitResult Structure (by ref)"))
  (`self.SwitchTrack` 2)
  (`KismetSystemLibrary.PrintString` "Track02"))

(event `self.Track03.OnComponentBeginOverlap`
  (params (OverlappedComponent :type "PrimitiveComponent Object Reference") (OtherActor :type "Actor Object Reference") (OtherComp :type "PrimitiveComponent Object Reference") (OtherBodyIndex :type Integer) (bFromSweep :type Boolean) (SweepResult :type "HitResult Structure (by ref)"))
  (`self.SwitchTrack` 3)
  (`KismetSystemLibrary.PrintString` "Track03"))

(event `self.Track04.OnComponentBeginOverlap`
  (params (OverlappedComponent :type "PrimitiveComponent Object Reference") (OtherActor :type "Actor Object Reference") (OtherComp :type "PrimitiveComponent Object Reference") (OtherBodyIndex :type Integer) (bFromSweep :type Boolean) (SweepResult :type "HitResult Structure (by ref)"))
  (`self.SwitchTrack` 4)
  (`KismetSystemLibrary.PrintString` "Track04"))

(event `self.Track05.OnComponentBeginOverlap`
  (params (OverlappedComponent :type "PrimitiveComponent Object Reference") (OtherActor :type "Actor Object Reference") (OtherComp :type "PrimitiveComponent Object Reference") (OtherBodyIndex :type Integer) (bFromSweep :type Boolean) (SweepResult :type "HitResult Structure (by ref)"))
  (`self.SwitchTrack` 5)
  (`KismetSystemLibrary.PrintString` "Track05"))

(event `self.Track06.OnComponentBeginOverlap`
  (params (OverlappedComponent :type "PrimitiveComponent Object Reference") (OtherActor :type "Actor Object Reference") (OtherComp :type "PrimitiveComponent Object Reference") (OtherBodyIndex :type Integer) (bFromSweep :type Boolean) (SweepResult :type "HitResult Structure (by ref)"))
  (`self.SwitchTrack` 6)
  (`KismetSystemLibrary.PrintString` "Track06"))

(fn `UserConstructionScript`)