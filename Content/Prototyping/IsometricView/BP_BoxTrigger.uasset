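; BP_BoxTrigger is a prototype trigger for the isometric view that toggles a linked bridge when a box of the matching Light or Dark type overlaps it.
; On overlap, it reads the actor's box type through BPI_BoxRef, compares it to TriggerType, then prints a debug message and calls OpenClose on the Bridge.
; The construction script colors its three cubes to show the trigger type.
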(event `self.Box.OnComponentBeginOverlap`
  (params (OverlappedComponent :type "PrimitiveComponent Object Reference") (OtherActor :type "Actor Object Reference") (OtherComp :type "PrimitiveComponent Object Reference") (OtherBodyIndex :type Integer) (bFromSweep :type Boolean) (SweepResult :type "HitResult Structure (by ref)"))
  (if (`KismetSystemLibrary.DoesImplementInterface` OtherActor "/Game/Prototyping/IsometricView/BPI_BoxRef.BPI_BoxRef_C")
    (bind _boxref (message `/Game/Prototyping/IsometricView/BPI_BoxRef.GetBoxRef` OtherActor))
    (if (`|EnumEquality` (`/Game/Prototyping/IsometricView/BP_Box.BoxType` _boxref) (`self.TriggerType`))
      (`KismetSystemLibrary.PrintString` "YAY! \n")
      (`/Game/Prototyping/IsometricView/BP_Bridge.OpenClose ` (`self.Bridge`)))))

(fn `GetBoxRef`
  (returns (BoxRef :type "/Game/Prototyping/IsometricView/BP_Box Object Reference"))
  (return null))

(fn `UserConstructionScript`
  (bind _cube1 (`self.Cube1`))
  (switch `/Game/Prototyping/IsometricView/ELightDark` (`self.TriggerType`)
    (:`NewEnumerator0`
      (`PrimitiveComponent.SetMaterial` _cube1 0 "/Game/Prototyping/IsometricView/MI_Light.MI_Light")
      (`PrimitiveComponent.SetMaterial` (`self.Cube2`) 0 "/Game/Prototyping/IsometricView/MI_Light.MI_Light")
      (`PrimitiveComponent.SetMaterial` (`self.Cube3`) 0 "/Game/Prototyping/IsometricView/MI_Light.MI_Light"))
    (:`NewEnumerator1`
      (`PrimitiveComponent.SetMaterial` _cube1 0 "/Game/Prototyping/IsometricView/MI_Dark.MI_Dark")
      (`PrimitiveComponent.SetMaterial` (`self.Cube2`) 0 "/Game/Prototyping/IsometricView/MI_Dark.MI_Dark")
      (`PrimitiveComponent.SetMaterial` (`self.Cube3`) 0 "/Game/Prototyping/IsometricView/MI_Dark.MI_Dark"))))