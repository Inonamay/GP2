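; BP_Box is a prototype cube of Light or Dark type that reacts to the player's light/dark world switch.
; The construction script sets its material and initial physics by type.
; At BeginPlay it binds to ThirdPersonCharacter's EDLightDark dispatcher and creates a dynamic material.
; Each world change enables physics and emissive glow when the world state is opposite the box's type, and disables both when they match.
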(event `self.ReceiveBeginPlay`
  (bind _asthird_person_character (cast `/Game/Prototyping/ThirdPersonStarter/ThirdPersonBP/Blueprints/ThirdPersonCharacter` (`GameplayStatics.GetPlayerPawn` 0)))
  (add `/Game/Prototyping/ThirdPersonStarter/ThirdPersonBP/Blueprints/ThirdPersonCharacter.ED_LightDark` _asthird_person_character (delegate `WorldState Change`))
  (bind _returnvalue (`PrimitiveComponent.CreateDynamicMaterialInstance` (`self.Cube`) 0 (`PrimitiveComponent.GetMaterial` (`self.Cube`) 0) "None"))
  (if (`|EnumEquality` (`self.BoxType`) "NewEnumerator0")
    (`MaterialInstanceDynamic.SetScalarParameterValue` _returnvalue "Emissive" 0.3)
    (else
      (`MaterialInstanceDynamic.SetScalarParameterValue` _returnvalue "Emissive" 0.0))))

(event `WorldState Change`
  (params (WorldState :type "/Game/Prototyping/IsometricView/ELightDark Enum" :default "NewEnumerator0"))
  (bind _cube (`self.Cube`))
  (bind _cube_2 (`self.Cube`))
  (if (`|EnumEquality` (`self.BoxType`) "NewEnumerator0")
    (switch `/Game/Prototyping/IsometricView/ELightDark` WorldState
      (:`NewEnumerator0`
        (`MaterialInstanceDynamic.SetScalarParameterValue` (stale `self.ReceiveBeginPlay` _returnvalue) "Emissive" 0.0)
        (`PrimitiveComponent.SetSimulatePhysics` _cube_2 false))
      (:`NewEnumerator1`
        (`MaterialInstanceDynamic.SetScalarParameterValue` (stale `self.ReceiveBeginPlay` _returnvalue) "Emissive" 0.3)
        (`PrimitiveComponent.SetSimulatePhysics` _cube_2 true)))
    (else
      (switch `/Game/Prototyping/IsometricView/ELightDark` WorldState
        (:`NewEnumerator0`
          (`MaterialInstanceDynamic.SetScalarParameterValue` (stale `self.ReceiveBeginPlay` _returnvalue) "Emissive" 0.3)
          (`PrimitiveComponent.SetSimulatePhysics` _cube true))
        (:`NewEnumerator1`
          (`MaterialInstanceDynamic.SetScalarParameterValue` (stale `self.ReceiveBeginPlay` _returnvalue) "Emissive" 0.0)
          (`PrimitiveComponent.SetSimulatePhysics` _cube false))))))

(fn `GetBoxRef`
  (returns (BoxRef :type "/Game/Prototyping/IsometricView/BP_Box Object Reference"))
  (return self))

(fn `UserConstructionScript`
  (bind _cube (`self.Cube`))
  (switch `/Game/Prototyping/IsometricView/ELightDark` (`self.BoxType`)
    (:`NewEnumerator0`
      (`PrimitiveComponent.SetMaterial` _cube 0 "/Game/Prototyping/IsometricView/MI_Light.MI_Light")
      (`PrimitiveComponent.SetSimulatePhysics` _cube true))
    (:`NewEnumerator1`
      (`PrimitiveComponent.SetMaterial` _cube 0 "/Game/Prototyping/IsometricView/MI_Dark.MI_Dark")
      (`PrimitiveComponent.SetSimulatePhysics` _cube false))))