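; BP_Block is a prototype block that slides its cube between two positions when the player switches the world between Light and Dark.
; On BeginPlay it binds to the ThirdPersonCharacter's light/dark event dispatcher.
; Each switch traces between two arrow markers and skips the move if a physics body is in the way.
; Otherwise a timeline lerps the cube from ArrowA to ArrowB for Light and reverses for Dark, without sweeping.
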(event `self.ReceiveBeginPlay`
  (bind _asthird_person_character (cast `/Game/Prototyping/ThirdPersonStarter/ThirdPersonBP/Blueprints/ThirdPersonCharacter` (`GameplayStatics.GetPlayerPawn` 0)))
  (add `/Game/Prototyping/ThirdPersonStarter/ThirdPersonBP/Blueprints/ThirdPersonCharacter.ED_LightDark` _asthird_person_character (delegate `ED_LightDark_Event_0`)))

(event `ED_LightDark_Event_0`
  (params (WorldState :type "/Game/Prototyping/IsometricView/ELightDark Enum" :default "NewEnumerator0"))
  (bind (_outhit _returnvalue) (`KismetSystemLibrary.LineTraceSingleForObjects` :`Start` (`SceneComponent.K2_GetComponentLocation` (`self.ArrowA`)) :`End` (`SceneComponent.K2_GetComponentLocation` (`self.ArrowB`)) :`ObjectTypes` (`|MakeArray` "ObjectTypeQuery4" :!type "EObjectTypeQuery Enum") :`DrawDebugType` "ForDuration"))
  (if (not _returnvalue)
    (switch `/Game/Prototyping/IsometricView/ELightDark` WorldState
      (:`NewEnumerator0`
        (bind (_direction _alpha) (`Timeline|TL_Move` :!via `PlayFromStart` :!label _label)
          (:`Update`
            (`SceneComponent.K2_SetWorldLocation` (`self.Cube`) (`KismetMathLibrary.VLerp` (`SceneComponent.K2_GetComponentLocation` (`self.ArrowA`)) (`SceneComponent.K2_GetComponentLocation` (`self.ArrowB`)) _alpha) false false))))
      (:`NewEnumerator1`
        (goto _label :!via `ReverseFromEnd`)))))

(fn `UserConstructionScript`)