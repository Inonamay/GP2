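; BP_TrackSwitch is a trigger volume that switches overlapping actors onto a different path spline and camera spline.
; On box overlap, it gets the splines from its referenced path and camera actors, if both are valid, and passes them to the entering actor through message calls.
; BeginPlay repeats the handoff after a short delay for every actor already overlapping, covering those that start inside the volume.
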(event `self.Box.OnComponentBeginOverlap`
  (params (OverlappedComponent :type "PrimitiveComponent Object Reference") (OtherActor :type "Actor Object Reference") (OtherComp :type "PrimitiveComponent Object Reference") (OtherBodyIndex :type Integer) (bFromSweep :type Boolean) (SweepResult :type "HitResult Structure (by ref)"))
  (if (and (`KismetSystemLibrary.IsValid` (`self.PathActorRef`)) (`KismetSystemLibrary.IsValid` (`self.CamerActorRef`)))
    (bind _splinecomponent (message `/Game/Prototyping/SplineStuff/BPI_SplineInterface.GetSpline` (`self.CamerActorRef`)))
    (message `/Game/Prototyping/SplineStuff/BPI_ComponentInterface.SetCamerSpline` OtherActor _splinecomponent)
    (bind _splinecomponent_2 (message `/Game/Prototyping/SplineStuff/BPI_SplineInterface.GetSpline` (`self.PathActorRef`)))
    (message `/Game/Prototyping/SplineStuff/BPI_ComponentInterface.SetPathSpline` OtherActor _splinecomponent_2)))

(event `self.ReceiveBeginPlay`
  (`KismetSystemLibrary.Delay` 0.2)
  (for _array_element (`self.GetOverlappingActors` null)
    (if (and (`KismetSystemLibrary.IsValid` (`self.PathActorRef`)) (`KismetSystemLibrary.IsValid` (`self.CamerActorRef`)))
      (bind _splinecomponent (message `/Game/Prototyping/SplineStuff/BPI_SplineInterface.GetSpline` (`self.CamerActorRef`)))
      (message `/Game/Prototyping/SplineStuff/BPI_ComponentInterface.SetCamerSpline` _array_element _splinecomponent)
      (bind _splinecomponent_2 (message `/Game/Prototyping/SplineStuff/BPI_SplineInterface.GetSpline` (`self.PathActorRef`)))
      (message `/Game/Prototyping/SplineStuff/BPI_ComponentInterface.SetPathSpline` _array_element _splinecomponent_2))))

(fn `UserConstructionScript`)