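; Tile-island lilypad that automatically carries the player along a spline to a lower layer during the day.
; Box overlap blocks movement, a timeline moves player and pad together, then the player snaps to MoveTo as the current tile.
; Night disables the trigger, runs the pad down the spline and hides it; day re-enables it and raises the pad at its start.
; Hover generates a path to MoveFrom; interact walks it.
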(event `self.DayNightTrigger.onNight`
  (params (time :type Integer))
  (bind _spline (`self.Spline`))
  ;[0 0 0] Hide/Show for Day and Night change
  (`PrimitiveComponent.SetCollisionEnabled` (`self.Box`) "NoCollision")
  (bind (_direction _alpha) (`Timeline|Timeline_0` :!via `PlayFromStart`)
    (:`Update`
      (`SceneComponent.K2_SetWorldLocation` (`self.Lillypad`) (`SplineComponent.GetLocationAtDistanceAlongSpline` _spline (* _alpha (`SplineComponent.GetSplineLength` _spline)) "World") false false))
    (:`Finished`
      (`KismetSystemLibrary.Delay` 0.5)
      (`SceneComponent.SetVisibility` (`self.Lillypad`) false false)
      (`SceneComponent.K2_SetWorldLocation` (`self.Lillypad`) (`KismetMathLibrary.MakeVector` (.x (`self.StartLocation`)) (.y (`self.StartLocation`)) (- (.z (`self.StartLocation`)) 50.0)) false false))))

(event `self.DayNightTrigger.onDay`
  (params (time :type Integer))
  ;[0 0 0] Hide/Show for Day and Night change
  (`PrimitiveComponent.SetCollisionEnabled` (`self.Box`) "QueryOnly")
  (`SceneComponent.SetVisibility` (`self.Lillypad`) true false)
  (bind (_direction _alpha) (`Timeline|Timeline_1` :!via `PlayFromStart`)
    (:`Update`
      (`SceneComponent.K2_SetWorldLocation` (`self.Lillypad`) (`KismetMathLibrary.VLerp` (`KismetMathLibrary.MakeVector` (.x (`self.StartLocation`)) (.y (`self.StartLocation`)) (- (.z (`self.StartLocation`)) 50.0)) (`self.StartLocation`) _alpha) false false))))

(event `self.ReceiveBeginPlay`
  ;[0 0 0] Begin Play
  (set `self.StartLocation` (`SceneComponent.K2_GetComponentLocation` (`self.Lillypad`))))

(event `self.Box.OnComponentBeginOverlap`
  (params (OverlappedComponent :type "PrimitiveComponent Object Reference") (OtherActor :type "Actor Object Reference") (OtherComp :type "PrimitiveComponent Object Reference") (OtherBodyIndex :type Integer) (bFromSweep :type Boolean) (SweepResult :type "HitResult Structure (by ref)"))
  (bind _output (`/Game/Core/BFL_Core.GetCharacter`))
  (bind _spline (`self.Spline`))
  (bind _moveto (`self.MoveTo`))
  ;[0 0 0] Move Player and Lily to new location
  (if (`|EnumEquality` (`/Game/DayNight/BFL_DayNight.GetTimeOfDay`) "Day")
    (`/Game/Movement/BFL_Movement.BlockOpenMovement` "NewEnumerator1")
    (set `/Game/Blueprints/Characters/GP2_PlayerCharacter.InterrupMovement` true (`/Game/Core/BFL_Core.GetCharacter`))
    (`KismetSystemLibrary.Delay` 0.5)
    (bind (_direction _alpha) (`Timeline|TL_MovePlyaer` :!via `PlayFromStart`)
      (:`Update`
        (bind _returnvalue (`SplineComponent.GetLocationAtDistanceAlongSpline` _spline (* _alpha (`SplineComponent.GetSplineLength` _spline)) "World"))
        (`self.K2_SetActorLocation` (`GameplayStatics.GetPlayerCharacter` 0) _returnvalue false true)
        (`SceneComponent.K2_SetWorldLocation` (`self.Lillypad`) _returnvalue false false))
      (:`Finished`
        ;[0 0 0] Set new Tile location for player
        (`self.K2_SetActorLocation` _output (`SceneComponent.K2_GetComponentLocation` (`/Game/Prototyping/TowerIsland/GroundSegment.WalkToPosition` _moveto)) false true)
        (`PlayerCharacter.SetCurrentTile` _output _moveto)
        (`KismetArrayLibrary.Array_Clear` (`/Game/Blueprints/Characters/GP2_PlayerCharacter.Path` _output))
        (set `/Game/Blueprints/Characters/GP2_PlayerCharacter.TargetTile` _moveto _output)
        (`/Game/Movement/BFL_Movement.BlockOpenMovement` "NewEnumerator0")
        (set `/Game/Blueprints/Characters/GP2_PlayerCharacter.InterrupMovement` false (`/Game/Core/BFL_Core.GetCharacter`))))))

(event `/Game/Prototyping/Interact/InteractInterface.Interact`
  (`/Game/Blueprints/Characters/GP2_PlayerCharacter.MoveAlongPath` (`/Game/Core/BFL_Core.GetCharacter`)))

(event `/Game/Prototyping/Interact/InteractInterface.Hover`
  (`PlayerCharacter.GeneratePathToWalkable` (`/Game/Core/BFL_Core.GetCharacter`) (`self.MoveFrom`)))

(fn `GetInteractTransform`
  (returns (Transform :type "Transform Structure"))
  (return))

(fn `UserConstructionScript`)