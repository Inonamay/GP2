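; BP_Camera_Child is a prototype camera actor for TowerIsland that tracks the player's height.
; It caches the ThirdPersonCharacter on BeginPlay, then each Tick matches its Z to the player's while leaving X and Y unchanged.
; It also applies the look-at rotation from player to camera to both itself and the player controller's control rotation, so both face along that line, away from the player.
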(event `self.ReceiveBeginPlay`
  (`parent.ReceiveBeginPlay`)
  (bind _asthird_person_character (cast `/Game/Prototyping/ThirdPersonStarter/ThirdPersonBP/Blueprints/ThirdPersonCharacter` (`GameplayStatics.GetPlayerPawn` 0)))
  (set `self.Player` _asthird_person_character))

(event `self.ReceiveTick`
  (params (DeltaSeconds :type "Float (single-precision)"))
  (bind (_returnvalue_x _returnvalue_y) (`KismetMathLibrary.BreakVector` (`self.K2_GetActorLocation`)))
  (bind (_returnvalue_x_2 _returnvalue_y_2 _returnvalue_z) (`KismetMathLibrary.BreakVector` (`self.K2_GetActorLocation` (`self.Player`))))
  (bind _returnvalue (`KismetMathLibrary.FindLookAtRotation` (`self.K2_GetActorLocation` (`self.Player`)) (`self.K2_GetActorLocation`)))
  (`self.K2_SetActorLocation` (`KismetMathLibrary.MakeVector` _returnvalue_x _returnvalue_y _returnvalue_z))
  (`self.K2_SetActorRotation` _returnvalue)
  (`Controller.SetControlRotation` (`GameplayStatics.GetPlayerController` 0) _returnvalue))

(fn `UserConstructionScript`
  (`parent.UserConstructionScript`))