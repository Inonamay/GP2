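; Tongue path piece for the Tower Island prototype that appears and becomes walkable only at night.
; DayNightTrigger events toggle Walkable.Blocked and play or reverse a timeline that scales the tongue root between zero and full size, starting blocked and reversed on BeginPlay.
; UpdatePathData sets the PathComponent's path type from the blocked state, and the WalkTo component supplies the interact transform.
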(event `self.ReceiveBeginPlay`
  (set `WalkableComponent.blocked` true (`self.Walkable`) :!label _label)
  (bind (_direction _alpha) (`Timeline|TL_Appear` :!via `Reverse` :!label _label_2)
    (:`Update`
      (`SceneComponent.SetRelativeScale3D` (`self.ToungeRoot`) (`KismetMathLibrary.VLerp` (0.0 0.0 0.0) (1.0 1.0 1.0) _alpha)))))

(event `self.DayNightTrigger.onDay`
  (params (time :type Integer))
  (goto _label))

(event `self.DayNightTrigger.onNight`
  (params (time :type Integer))
  (set `WalkableComponent.blocked` false (`self.Walkable`))
  (goto _label_2))

(event `/Game/Movement/PathInterface.UpdatePathData`
  (set `/Game/Movement/PathComponent.PathType` (select `bool` (`WalkableComponent.blocked` (`self.Walkable`)) :`false` "NewEnumerator0" :`true` "NewEnumerator1" :!type "/Game/Movement/E_PathPointTypes Enum") (`self.PathComponent`)))

(fn `GetInteractTransform`
  (returns (Transform :type "Transform Structure"))
  (return (`SceneComponent.K2_GetComponentToWorld` (`self.WalkTo`))))

(fn `GetPathPoint`
  (returns (PathPoint :type "Vector Structure"))
  (return (0.0 0.0 0.0)))

(fn `UserConstructionScript`)