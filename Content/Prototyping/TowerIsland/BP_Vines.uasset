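; BP_Vines is a prototype TowerIsland vine actor whose interactable state depends on the time of day.
; The construction script uses IsDayVines to make its InteractComponent interactable in either day or night, and sets the initial cube material to match.
; DayNightTrigger's OnDay and OnNight events read those flags and swap the cube between the vine material when interactable and the blocker material otherwise.
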(event `self.DayNightTrigger.onDay`
  (params (time :type Integer))
  (bind _cube (`self.Cube`))
  (if (`/Game/Prototyping/Interact/InteractComponent.Interactable Day` (`self.InteractComponent`))
    (`PrimitiveComponent.SetMaterial` _cube 0 "/Game/Prototyping/IsometricView/MI_Vine.MI_Vine" :!label _label)
    (else
      (`PrimitiveComponent.SetMaterial` _cube 0 "/Game/Prototyping/IsometricView/MI_Blocker.MI_Blocker" :!label _label_2))))

(event `self.DayNightTrigger.onNight`
  (params (time :type Integer))
  (if (`/Game/Prototyping/Interact/InteractComponent.Interactable Night` (`self.InteractComponent`))
    (goto _label)
    (else
      (goto _label_2))))

(fn `UserConstructionScript`
  (bind _cube (`self.Cube`))
  (bind _interactcomponent (`self.InteractComponent`))
  (if (`self.IsDayVines`)
    (`PrimitiveComponent.SetMaterial` _cube 0 "/Game/Prototyping/IsometricView/MI_Vine.MI_Vine")
    (set `/Game/Prototyping/Interact/InteractComponent.Interactable Day` true _interactcomponent)
    (set `/Game/Prototyping/Interact/InteractComponent.Interactable Night` false _interactcomponent)
    (else
      (`PrimitiveComponent.SetMaterial` _cube 0 "/Game/Prototyping/IsometricView/MI_Blocker.MI_Blocker")
      (set `/Game/Prototyping/Interact/InteractComponent.Interactable Day` false _interactcomponent)
      (set `/Game/Prototyping/Interact/InteractComponent.Interactable Night` true _interactcomponent))))