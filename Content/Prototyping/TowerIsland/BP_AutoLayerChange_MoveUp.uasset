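; Mushroom interactable in the TowerIsland prototype that carries the player to another tile, apparently a layer up.
; Interacting plays a timeline that teleports the player along a spline each update, then snaps them to the MoveTo tile's walk position and sets it as current tile after a short delay.
; A DayNightTrigger swaps the mushroom mesh between day and night versions; the InteractComponent day/night checks are unconnected.
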(event `self.ReceiveBeginPlay`)

(event `self.DayNightTrigger.onDay`
  (params (time :type Integer))
  (`StaticMeshComponent.SetStaticMesh` (`self.Cylinder`) "/Game/Art_Testing/Berries/Shroom_Day.Shroom_Day"))

(event `/Game/Prototyping/Interact/InteractInterface.Interact`
  (bind _output (`/Game/Core/BFL_Core.GetCharacter`))
  (bind _moveto (`self.MoveTo`))
  (bind _spline (`self.Spline`))
  (bind (_direction _alpha) (`Timeline|TL_MovePlyaer` :!via `PlayFromStart`)
    (:`Update`
      (`self.K2_SetActorLocation` (`GameplayStatics.GetPlayerCharacter` 0) (`SplineComponent.GetLocationAtDistanceAlongSpline` _spline (* _alpha (`SplineComponent.GetSplineLength` _spline)) "World") false true))
    (:`Finished`
      (`self.K2_SetActorLocation` _output (`SceneComponent.K2_GetComponentLocation` (`/Game/Prototyping/TowerIsland/GroundSegment.WalkToPosition` _moveto)) false true)
      (`KismetSystemLibrary.Delay` 0.3)
      (`PlayerCharacter.SetCurrentTile` _output _moveto))))

(event `self.DayNightTrigger.onNight`
  (params (time :type Integer))
  (`StaticMeshComponent.SetStaticMesh` (`self.Cylinder`) "/Game/Art_Testing/Berries/Shroom_Night.Shroom_Night"))

(fn `GetInteractTransform`
  (returns (Transform :type "Transform Structure"))
  (return))

(fn `UserConstructionScript`)