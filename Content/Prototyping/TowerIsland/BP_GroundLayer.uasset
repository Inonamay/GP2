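; Ground layer for the TowerIsland prototype that builds a spline ring of GroundSegment pieces.
; GenerateCircle lays points from radius and segment spacing, and GenerateSegmentActors spawns a segment per span with a raised, sideways-offset walk-to transform, itself as controller, and initial connections.
; The construction script re-fits existing segments to the spline by sending endpoints, tangents and scales.
; GenerateSegments is a child-actor variant using SegmentData meshes, with no live caller here.
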(fn `Delete`
  (for _array_element (`self.SegmentList`)
    (`self.K2_DestroyActor` _array_element))
  (`self.K2_DestroyActor`))

(fn `GenerateCircle`
  (bind _returnvalue (`KismetMathLibrary.Round` (/ (* (`self.Radius`) (`KismetMathLibrary.MultiplyByPi` 2.0)) (`self.SegmentSpacing`))))
  (`|ExecutionSequence`
    (:`then_0`
      (`KismetArrayLibrary.Array_Clear` (`self.SegmentData`)))
    (:`then_1`
      (`SplineComponent.ClearSplinePoints` (`self.Spline`) true)
      (for _index (range _returnvalue)
        (bind _returnvalue_2 (* -1 (* _index (/ 360.0 (`KismetMathLibrary.Conv_IntToDouble` _returnvalue)))))
        (`SplineComponent.AddSplinePoint` (`self.Spline`) (* (`KismetMathLibrary.MakeVector` (`KismetMathLibrary.DegCos` _returnvalue_2) (`KismetMathLibrary.DegSin` _returnvalue_2)) (`self.Radius`)) "Local" true)
        ;[1 1 1] Add Emtpy Data Entry
        (`KismetArrayLibrary.Array_Add` (`self.SegmentData`))))))

(fn `GenerateSegmentActors`
  (bind _spline (`self.Spline`))
  (bind _segmentlist (`self.SegmentList`))
  (bind _splinemeshscale (`self.SplineMeshScale`))
  (`|ExecutionSequence`
    (:`then_0`
      (for _array_element _segmentlist
        (`self.K2_DestroyActor` _array_element))
      (`KismetArrayLibrary.Array_Clear` _segmentlist)
      (`|ExecutionSequence`
        (:`then_0`
          (for _index (range (`SplineComponent.GetNumberOfSplinePoints` _spline))
            (bind _returnvalue (`|SpawnActorFromClass` "/Game/Prototyping/TowerIsland/GroundSegment.GroundSegment_C" (`KismetMathLibrary.MakeTransform` (0.0 0.0 0.0)) "AlwaysSpawn" "OverrideRootScale" null null))
            (bind (_returnvalue_x _returnvalue_y) (`KismetMathLibrary.BreakVector` (`SplineComponent.GetScaleAtSplinePoint` _spline _index)))
            (bind _returnvalue_2 (+ _index 1))
            (bind (_returnvalue_x_2 _returnvalue_y_2) (`KismetMathLibrary.BreakVector` (`SplineComponent.GetScaleAtSplinePoint` _spline _returnvalue_2)))
            (message `/Game/Prototyping/SplineStuff/SplineMeshInterface.SetStartAndEnd` _returnvalue (`SplineComponent.GetLocationAtSplinePoint` _spline _index "World") (`SplineComponent.GetTangentAtSplinePoint` _spline _index "World") (* _splinemeshscale (`KismetMathLibrary.MakeVector2D` _returnvalue_y 1.0)) (`SplineComponent.GetLocationAtSplinePoint` _spline _returnvalue_2 "World") (`SplineComponent.GetTangentAtSplinePoint` _spline _returnvalue_2 "World") (* _splinemeshscale (`KismetMathLibrary.MakeVector2D` _returnvalue_y_2 1.0)))
            (bind _returnvalue_3 (`SplineComponent.GetDistanceAlongSplineAtSplinePoint` _spline _returnvalue_2))
            (bind _returnvalue_4 (- _returnvalue_3 (/ (- _returnvalue_3 (`SplineComponent.GetDistanceAlongSplineAtSplinePoint` _spline _index)) 2.0)))
            (bind _returnvalue_5 (`KismetMathLibrary.ComposeRotators` (`KismetMathLibrary.Conv_VectorToRotator` (`SplineComponent.GetDirectionAtDistanceAlongSpline` _spline _returnvalue_4 "World")) (struct :`Yaw` 90.0)))
            (message `/Game/Prototyping/Interact/InteractInterface.SetWalkToTransform` _returnvalue (`KismetMathLibrary.MakeTransform` (+ (`SplineComponent.GetLocationAtDistanceAlongSpline` _spline _returnvalue_4 "World") (0.0 0.0 300.0) (* (`KismetMathLibrary.Conv_RotatorToVector` _returnvalue_5) 150.0)) _returnvalue_5))
            (`KismetArrayLibrary.Array_AddUnique` (`self.SegmentList`) _returnvalue)))
        (:`then_1`
          ;[1 1 1] Set self as controller on segments
          (`self.UpdateControllerOnSegments`))))
    (:`then_1`
      (`/Game/Prototyping/TowerIsland/BFL_TowerBuilder.SetInitialConnections` _segmentlist))))

(fn `GenerateSegments`
  (bind _spline (`self.Spline`))
  (bind _segments (`self.Segments`))
  (bind _splinemeshscale (`self.SplineMeshScale`))
  (bind (_arrayindex _arrayelement) (`/Engine/EditorBlueprintResources/StandardMacros.ReverseForEachLoop` _segments)
    (:`LoopBody`
      (`ActorComponent.K2_DestroyComponent` _arrayelement))
    (:`Completed`
      (`KismetArrayLibrary.Array_Clear` _segments)
      (for _index (range (`SplineComponent.GetNumberOfSplinePoints` _spline))
        (bind _returnvalue (`AddComponent|NODE_AddChildActorComponent-0`))
        (bind _childactor (`ChildActorComponent.ChildActor` _returnvalue))
        (bind (_returnvalue_x _returnvalue_y) (`KismetMathLibrary.BreakVector` (`SplineComponent.GetScaleAtSplinePoint` _spline _index)))
        (bind _returnvalue_2 (+ _index 1))
        (bind (_returnvalue_x_2 _returnvalue_y_2) (`KismetMathLibrary.BreakVector` (`SplineComponent.GetScaleAtSplinePoint` _spline _returnvalue_2)))
        (message `/Game/Prototyping/SplineStuff/SplineMeshInterface.SetStartAndEnd` _childactor (`SplineComponent.GetLocationAtSplinePoint` _spline _index "World") (`SplineComponent.GetTangentAtSplinePoint` _spline _index "World") (* _splinemeshscale (`KismetMathLibrary.MakeVector2D` _returnvalue_y 1.0)) (`SplineComponent.GetLocationAtSplinePoint` _spline _returnvalue_2 "World") (`SplineComponent.GetTangentAtSplinePoint` _spline _returnvalue_2 "World") (* _splinemeshscale (`KismetMathLibrary.MakeVector2D` _returnvalue_y_2 1.0)))
        (bind _asground_segment (cast `/Game/Prototyping/TowerIsland/GroundSegment` _childactor))
        (bind _output_mesh (break `/Game/Prototyping/TowerIsland/STR_GroundSegmentData` (`|GetArrayItem` (`self.SegmentData`) _index)))
        (`StaticMeshComponent.SetStaticMesh` (`/Game/Prototyping/TowerIsland/GroundSegment.SplineMesh` _asground_segment) _output_mesh)
        (bind _returnvalue_3 (`SplineComponent.GetDistanceAlongSplineAtSplinePoint` _spline _returnvalue_2))
        (bind _returnvalue_4 (- _returnvalue_3 (/ (- _returnvalue_3 (`SplineComponent.GetDistanceAlongSplineAtSplinePoint` _spline _index)) 2.0)))
        (bind _returnvalue_5 (`KismetMathLibrary.ComposeRotators` (`KismetMathLibrary.Conv_VectorToRotator` (`SplineComponent.GetDirectionAtDistanceAlongSpline` _spline _returnvalue_4 "World")) (struct :`Yaw` 90.0)))
        (message `/Game/Prototyping/Interact/InteractInterface.SetWalkToTransform` _childactor (`KismetMathLibrary.MakeTransform` (+ (`SplineComponent.GetLocationAtDistanceAlongSpline` _spline _returnvalue_4 "World") (0.0 0.0 300.0) (* (`KismetMathLibrary.Conv_RotatorToVector` _returnvalue_5) 150.0)) _returnvalue_5))
        (`KismetArrayLibrary.Array_AddUnique` (`self.Segments`) _returnvalue)))))

(fn `GetSpline`
  (returns (SPlineComponent :type "SplineComponent Object Reference"))
  (return (`self.Spline`)))

(fn `Regenerate`
  (`self.GenerateCircle`))

(fn `UpdateControllerOnSegments`
  (for _array_element (`self.SegmentList`)
    (bind _asground_segment (cast `/Game/Prototyping/TowerIsland/GroundSegment` _array_element))
    (set `/Game/Prototyping/TowerIsland/GroundSegment.Controller` self _asground_segment)))

(fn `UserConstructionScript`
  (bind _spline (`self.Spline`))
  (bind _splinemeshscale (`self.SplineMeshScale`))
  (for _index (range (`SplineComponent.GetNumberOfSplinePoints` _spline))
    (bind (_returnvalue_x _returnvalue_y) (`KismetMathLibrary.BreakVector` (`SplineComponent.GetScaleAtSplinePoint` _spline _index)))
    (bind _returnvalue (+ _index 1))
    (bind (_returnvalue_x_2 _returnvalue_y_2) (`KismetMathLibrary.BreakVector` (`SplineComponent.GetScaleAtSplinePoint` _spline _returnvalue)))
    (message `/Game/Prototyping/SplineStuff/SplineMeshInterface.SetStartAndEnd` (`|GetArrayItem` (`self.SegmentList`) _index) (`SplineComponent.GetLocationAtSplinePoint` _spline _index "World") (`SplineComponent.GetTangentAtSplinePoint` _spline _index "World") (* _splinemeshscale (`KismetMathLibrary.MakeVector2D` _returnvalue_y 1.0)) (`SplineComponent.GetLocationAtSplinePoint` _spline _returnvalue "World") (`SplineComponent.GetTangentAtSplinePoint` _spline _returnvalue "World") (* _splinemeshscale (`KismetMathLibrary.MakeVector2D` _returnvalue_y_2 1.0)))))