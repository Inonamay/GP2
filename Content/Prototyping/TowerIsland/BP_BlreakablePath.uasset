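; A breakable path Blueprint in the TowerIsland prototype that gives way after being crossed and rebuilds over day/night turns.
; Leaving the box trigger marks it Broken and plays a timeline; entering only swaps the cube's material.
; Day and night changes count rebuild turns, then reverse the timeline, which lerps the cube between two arrows; Broken is never cleared and the delay is zeroed.
; Interact teleports the player to WalkToLocation.
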(event `self.ReceiveBeginPlay`)

(event `self.DayNightTrigger.onDay`
  (params (time :type Integer))
  (if (`self.Broken`) :!label _label
    (bind _result (`/Engine/EditorBlueprintResources/StandardMacros.IncrementInt` (`self.RebuildingTurns`))
      (:`  `
        (if (>= _result (`self.RebuildTurnDelay`))
          (set `self.RebuildTurnDelay` 0)
          (set `self.RebuildingTurns` 0)
          (bind (_direction _alpha) (`Timeline|TL_Move` :!via `ReverseFromEnd` :!label _label_2)
            (:`Update`
              (`SceneComponent.K2_SetWorldLocation` (`self.Cube`) (`KismetMathLibrary.VLerp` (`SceneComponent.K2_GetComponentLocation` (`self.ArrowA`)) (`SceneComponent.K2_GetComponentLocation` (`self.ArrowB`)) _alpha) false false))))))))

(event `self.DayNightTrigger.onNight`
  (params (time :type Integer))
  (goto _label))

(event `/Game/Prototyping/Interact/InteractInterface.Interact`
  (`self.K2_SetActorLocation` (`GameplayStatics.GetPlayerCharacter` 0) (`SceneComponent.K2_GetComponentLocation` (`self.WalkToLocation`)) false true))

(event `self.Box.OnComponentBeginOverlap`
  (params (OverlappedComponent :type "PrimitiveComponent Object Reference") (OtherActor :type "Actor Object Reference") (OtherComp :type "PrimitiveComponent Object Reference") (OtherBodyIndex :type Integer) (bFromSweep :type Boolean) (SweepResult :type "HitResult Structure (by ref)"))
  (`PrimitiveComponent.SetMaterial` (`self.Cube`) 0 "/Game/Prototyping/IsometricView/MI_Light.MI_Light"))

(event `self.Box.OnComponentEndOverlap`
  (params (OverlappedComponent :type "PrimitiveComponent Object Reference") (OtherActor :type "Actor Object Reference") (OtherComp :type "PrimitiveComponent Object Reference") (OtherBodyIndex :type Integer))
  (`PrimitiveComponent.SetMaterial` (`self.Cube`) 0 "/Game/Prototyping/IsometricView/MI_Blocker.MI_Blocker")
  (set `self.Broken` true)
  (goto _label_2 :!via `PlayFromStart`))

(fn `UserConstructionScript`)