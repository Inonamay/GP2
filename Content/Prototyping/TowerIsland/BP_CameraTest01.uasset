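; BP_CameraTest01 is a prototype camera test for TowerIsland that snaps the referenced ZeCamera to the world origin on BeginPlay.
; A timeline that lerps the camera from its current location to the origin is present but never runs.
; An unused spline lookup finds the point on CameraSpline closest to a position ahead of the player character, and the MovingEnded event is empty.
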(event `self.ReceiveBeginPlay`
  (`SceneComponent.K2_SetWorldLocation` (`Actor.RootComponent` (`self.ZeCamera`)) (0.0 0.0 0.0) false false))

(event `/Game/Movement/MovementInterface.MovingEnded`)

(fn `UserConstructionScript`)