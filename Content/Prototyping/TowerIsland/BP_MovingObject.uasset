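; Tower Island prototype hazard: an animated mesh actor that ping-pongs along spline points and restarts the stage when the player's character overlaps its collider.
; MoveOnStep selects whether it advances one point per MovedOneStep event or per day/night change, and sets the cube material.
; Timelines lerp each move, then the skeletal mesh turns toward the next point; ResetFloor returns it to its start.
; A particle repeatedly sweeps the spline back and forth, pausing between passes.
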(event `self.ReceiveBeginPlay`
  (bind _animationdrivencomponent (`self.AnimationDrivenComponent`))
  (set `/Game/AnimationSystem/AnimationDrivenComponent.Driver` (`self.AnimationDriverComponent`) _animationdrivencomponent)
  (message `/Game/AnimationSystem/AnimationSystemInterface.PlayAnimation` _animationdrivencomponent "NewEnumerator1" -1)
  (set `self.Current` (`self.StartSplineIndex`))
  (`/Engine/EditorBlueprintResources/StandardMacros.FlipFlop` :!label _label
    (:`A`
      (bind (_direction _alpha) (`Timeline|Timeline_0` :!via `PlayFromStart` :!label _label_2)
        (:`Update`
          (`SceneComponent.K2_SetRelativeLocation` (`self.ParticleSystem`) (`SplineComponent.GetLocationAtDistanceAlongSpline` (`self.Spline`) (* _alpha (`SplineComponent.GetSplineLength` (`self.Spline`))) "Local") false false))
        (:`Finished`
          (`KismetSystemLibrary.Delay` 10.0)
          (goto _label))))
    (:`B`
      (goto _label_2 :!via `ReverseFromEnd`))))

(event `/Game/Movement/MovementInterface.MovedOneStep`
  (bind _current (`self.Current`))
  (bind _spline (`self.Spline`))
  (bind _spline_2 (`self.Spline`))
  (bind _spline_3 (`self.Spline`))
  (bind _current_2 (`self.Current`))
  (bind _skeletalmesh (`self.SkeletalMesh`))
  ;[0 0 0] Move on Step
  (if (`self.MoveOnStep`)
    (message `/Game/AnimationSystem/AnimationSystemInterface.PlayAnimation` (`self.AnimationDrivenComponent`) "NewEnumerator2" 0 :!label _label_3)
    (bind (_direction _alpha) (`Timeline|TL_Move` :!via `PlayFromStart`)
      (:`Update`
        (if (`self.isReverse`)
          (`SceneComponent.K2_SetWorldLocation` (`self.Cube`) (`KismetMathLibrary.VLerp` (`SplineComponent.GetLocationAtSplinePoint` _spline _current "World") (`SplineComponent.GetLocationAtSplinePoint` _spline (- _current 1) "World") _alpha) false false)
          (else
            (`SceneComponent.K2_SetWorldLocation` (`self.Cube`) (`KismetMathLibrary.VLerp` (`SplineComponent.GetLocationAtSplinePoint` _spline_3 _current_2 "World") (`SplineComponent.GetLocationAtSplinePoint` _spline_3 (+ _current_2 1) "World") _alpha) false false))))
      (:`Finished`
        (`|ExecutionSequence`
          (:`then_0`
            (if (`self.isReverse`)
              (bind _result (`/Engine/EditorBlueprintResources/StandardMacros.DecrementInt` (`self.Current`))
                (:`  `
                  (if (<= _result 0)
                    (set `self.isReverse` false)
                    (`SceneComponent.K2_SetWorldRotation` _skeletalmesh (`KismetMathLibrary.MakeRotator` (.roll (`KismetMathLibrary.FindLookAtRotation` (`SceneComponent.K2_GetComponentLocation` (`self.SkeletalMesh`)) (`SplineComponent.GetLocationAtSplinePoint` _spline_2 (+ (`self.Current`) 1) "World"))) (.pitch (`KismetMathLibrary.FindLookAtRotation` (`SceneComponent.K2_GetComponentLocation` (`self.SkeletalMesh`)) (`SplineComponent.GetLocationAtSplinePoint` _spline_2 (+ (`self.Current`) 1) "World"))) (- (.yaw (`KismetMathLibrary.FindLookAtRotation` (`SceneComponent.K2_GetComponentLocation` (`self.SkeletalMesh`)) (`SplineComponent.GetLocationAtSplinePoint` _spline_2 (+ (`self.Current`) 1) "World"))) 90.0)) false false :!label _label_4)
                    (else
                      (`SceneComponent.K2_SetWorldRotation` _skeletalmesh (`KismetMathLibrary.MakeRotator` (.roll (`KismetMathLibrary.FindLookAtRotation` (`SceneComponent.K2_GetComponentLocation` (`self.SkeletalMesh`)) (`SplineComponent.GetLocationAtSplinePoint` _spline_2 (- (`self.Current`) 1) "World"))) (.pitch (`KismetMathLibrary.FindLookAtRotation` (`SceneComponent.K2_GetComponentLocation` (`self.SkeletalMesh`)) (`SplineComponent.GetLocationAtSplinePoint` _spline_2 (- (`self.Current`) 1) "World"))) (- (.yaw (`KismetMathLibrary.FindLookAtRotation` (`SceneComponent.K2_GetComponentLocation` (`self.SkeletalMesh`)) (`SplineComponent.GetLocationAtSplinePoint` _spline_2 (- (`self.Current`) 1) "World"))) 90.0)) false false :!label _label_5)))))
              (else
                (bind _result_2 (`/Engine/EditorBlueprintResources/StandardMacros.IncrementInt` (`self.Current`))
                  (:`  `
                    (if (>= _result_2 (- (`SplineComponent.GetNumberOfSplinePoints` _spline_2) 1))
                      (set `self.isReverse` true)
                      (goto _label_5)
                      (else
                        (goto _label_4))))))))
          (:`then_1`
            (message `/Game/AnimationSystem/AnimationSystemInterface.PlayAnimation` (`self.AnimationDrivenComponent`) "NewEnumerator1" -1)))))))

(event `self.DayNightTrigger.onNight`
  (params (time :type Integer))
  ;[0 0 0] Move on DayNightTrigger
  (if (not (`self.MoveOnStep`)) :!label _label_6
    (goto _label_3)))

(event `self.DayNightTrigger.onDay`
  (params (time :type Integer))
  ;[0 0 0] Move on DayNightTrigger
  (goto _label_6))

(event `/Game/Core/BPI_LevelReset.ResetFloor`
  (bind _spline (`self.Spline`))
  ;[0 0 0] Reset location
  (message `/Game/AnimationSystem/AnimationSystemInterface.PlayAnimation` (`self.AnimationDrivenComponent`) "NewEnumerator2" 0)
  (bind (_direction _alpha) (`Timeline|Timeline_1` :!via `PlayFromStart`)
    (:`Update`
      (`SceneComponent.K2_SetWorldLocation` (`self.Cube`) (`KismetMathLibrary.VLerp` (`SplineComponent.GetLocationAtSplinePoint` _spline (`self.Current`) "World") (`SplineComponent.GetLocationAtSplinePoint` _spline (`self.StartSplineIndex`) "World") _alpha) false false))
    (:`Finished`
      (set `self.Current` (`self.StartSplineIndex`))
      (set `self.isReverse` false))))

(event `self.PlayerColloder.OnComponentBeginOverlap`
  (params (OverlappedComponent :type "PrimitiveComponent Object Reference") (OtherActor :type "Actor Object Reference") (OtherComp :type "PrimitiveComponent Object Reference") (OtherBodyIndex :type Integer) (bFromSweep :type Boolean) (SweepResult :type "HitResult Structure (by ref)"))
  (bind _output (`/Game/Core/BFL_Core.GetCharacter`))
  ;[0 0 0 1 24] Reset player position when hit
  (if (== (`GameplayStatics.GetObjectClass` OtherActor) (`GameplayStatics.GetObjectClass` _output))
    (`/Game/Blueprints/Characters/GP2_PlayerCharacter.Restart Stage` _output)))

(fn `GetAnimationMesh`
  (returns (Result :type "SkeletalMeshComponent Object Reference"))
  (return (`self.SkeletalMesh`)))

(fn `UserConstructionScript`
  (if (`self.MoveOnStep`)
    (`PrimitiveComponent.SetMaterial` (`self.Cube`) 0 "/Game/Prototyping/TowerIsland/MI_Tower01.MI_Tower01")))