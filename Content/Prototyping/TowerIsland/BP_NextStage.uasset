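; BP_NextStage is a stage-exit trigger in the TowerIsland prototype that lets the player advance once they hold enough key items.
; On overlap, it moves the character to the MoveTo tile's walk position and starts a CameraSpline camera move.
; After a short delay it sets that tile as current and starting tile and resets key items, otherwise printing a warning.
; The construction script displays the required key count on a text render.
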(event `self.CollisionComponent.OnComponentBeginOverlap`
  (params (OverlappedComponent :type "PrimitiveComponent Object Reference") (OtherActor :type "Actor Object Reference") (OtherComp :type "PrimitiveComponent Object Reference") (OtherBodyIndex :type Integer) (bFromSweep :type Boolean) (SweepResult :type "HitResult Structure (by ref)"))
  (bind _output (`/Game/Core/BFL_Core.GetCharacter`))
  (bind _output_2 (`/Game/Core/BFL_Core.GetCharacter`))
  (bind _moveto (`self.MoveTo`))
  ;[0 0 0] Move player and start camera movement
  (if (>= (`/Game/Blueprints/Characters/GP2_PlayerCharacter.KeyItems` (`/Game/Core/BFL_Core.GetCharacter`)) (`self.KeyItemsNeeded`))
    (`self.K2_SetActorLocation` _output (`SceneComponent.K2_GetComponentLocation` (`/Game/Prototyping/TowerIsland/GroundSegment.WalkToPosition` _moveto)) false false)
    (`/Game/Prototyping/Camera/CameraSpline.Move Camera` (`self.cameraSpline`))
    (`KismetSystemLibrary.Delay` 1.0)
    (`PlayerCharacter.SetCurrentTile` _output _moveto)
    (set `/Game/Blueprints/Characters/GP2_PlayerCharacter.KeyItems` 0 _output_2)
    (set `PlayerCharacter.startingTile` _moveto _output_2)
    (else
      (`KismetSystemLibrary.PrintString` "Not enough Key Items"))))

(fn `UserConstructionScript`
  (`TextRenderComponent.K2_SetText` (`self.TextRender1`) (`|FormatText` "Keys: {Amount}" (`self.KeyItemsNeeded`))))