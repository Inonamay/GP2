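; BP_AutoLayerChange is a prototype interactable that carries the player along a spline to another position, with availability shown by day or night.
; On Interact, a timeline teleports player 0 along the spline each update, then snaps them to the MoveTo target's WalkToPosition.
; At BeginPlay and on DayNightTrigger events, the Cylinder switches between vine and blocker materials based on InteractComponent's day or night interactable flag, with BeginPlay assuming day.
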(event `/Game/Prototyping/Interact/InteractInterface.Interact`
  (bind _spline (`self.Spline`))
  (bind (_direction _alpha) (`Timeline|TL_MovePlyaer` :!via `PlayFromStart`)
    (:`Update`
      (`self.K2_SetActorLocation` (`GameplayStatics.GetPlayerCharacter` 0) (`SplineComponent.GetLocationAtDistanceAlongSpline` _spline (* _alpha (`SplineComponent.GetSplineLength` _spline)) "World") false true))
    (:`Finished`
      (`self.K2_SetActorLocation` (`GameplayStatics.GetPlayerCharacter` 0) (`SceneComponent.K2_GetComponentLocation` (`/Game/Prototyping/TowerIsland/GroundSegment.WalkToPosition` (`self.MoveTo`))) false true))))

(event `self.ReceiveBeginPlay`
  (bind _cylinder (`self.Cylinder`))
  (if (`/Game/Prototyping/Interact/InteractComponent.Interactable Day` (`self.InteractComponent`)) :!label _label
    (`PrimitiveComponent.SetMaterial` _cylinder 0 "/Game/Prototyping/IsometricView/MI_Vine.MI_Vine" :!label _label_2)
    (else
      (`PrimitiveComponent.SetMaterial` _cylinder 0 "/Game/Prototyping/IsometricView/MI_Blocker.MI_Blocker" :!label _label_3))))

(event `self.DayNightTrigger.onDay`
  (params (time :type Integer))
  (goto _label))

(event `self.DayNightTrigger.onNight`
  (params (time :type Integer))
  (if (`/Game/Prototyping/Interact/InteractComponent.Interactable Night` (`self.InteractComponent`))
    (goto _label_2)
    (else
      (goto _label_3))))

(fn `UserConstructionScript`)